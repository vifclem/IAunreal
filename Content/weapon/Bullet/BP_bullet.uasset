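; Bullet actor that damages whatever it hits, then destroys itself.
; On hit, it applies damage and an inward impulse direction to destructible actors, and subtracts random Life from BP_ThirdPersonCharacter, giving it a short lifespan at zero.
; A small sphere trace also runs, but its result is unused.
; Debug prints re-roll their random values, so they do not report the damage dealt.
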(event `self.ReceiveHit`
  (params (MyComp :type "PrimitiveComponent Object Reference") (Other :type "Actor Object Reference") (OtherComp :type "PrimitiveComponent Object Reference") (bSelfMoved :type Boolean) (HitLocation :type "Vector Structure") (HitNormal :type "Vector Structure") (NormalImpulse :type "Vector Structure") (Hit :type "HitResult Structure (by ref)"))
  (bind (_bblockinghit _binitialoverlap _time _distance _location _impactpoint _normal _impactnormal _physmat _hitactor) (`GameplayStatics.BreakHitResult` Hit))
  (bind _returnvalue (`KismetMathLibrary.RandomFloatInRange` 0.5 3.0))
  (`KismetSystemLibrary.SphereTraceSingle` (0.0 0.0 0.0) (0.0 0.0 0.0) 0.5 "TraceTypeQuery1" false (`self.Actors to Ignore`))
  (`|ExecutionSequence`
    (:`then_0`
      (bind _asdestructible_actor (cast `DestructibleActor` _hitactor)
        (:`then`
          (`DestructibleComponent.ApplyDamage` (`DestructibleActor.DestructibleComponent` _asdestructible_actor) 0.0 _impactpoint (* _impactnormal -1.0) 0.0)
          (`KismetSystemLibrary.PrintText` (`|FormatText` (`KismetTextLibrary.Conv_StringToText` (`KismetSystemLibrary.GetDisplayName` _hitactor)) _returnvalue)))
        (:`CastFailed`
          _)))
    (:`then_1`
      (bind _asbp_third_person_character (cast `/Game/ThirdPerson/Blueprints/BP_ThirdPersonCharacter` _hitactor)
        (:`then`
          (bind _output_get (set `/Game/ThirdPerson/Blueprints/BP_ThirdPersonCharacter.Life` (- (`/Game/ThirdPerson/Blueprints/BP_ThirdPersonCharacter.Life` _asbp_third_person_character) _returnvalue) _asbp_third_person_character))
          (`KismetSystemLibrary.PrintText` (`|FormatText` "" (`KismetTextLibrary.Conv_StringToText` (`KismetSystemLibrary.GetDisplayName` _hitactor)) _returnvalue))
          (if (<= _output_get 0.0)
            (`self.SetLifeSpan` _asbp_third_person_character 1.5)))
        (:`CastFailed`
          _))))
  (`self.K2_DestroyActor`))

(fn `UserConstructionScript`)